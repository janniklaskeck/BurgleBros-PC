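; BP_Level is a room or level actor whose Box component is fitted to a square tiled floor.
; The construction script derives the box's X and Y extents from FloorWidth and TileWidth.
; It also offsets the box in X and Y using the same values and a fixed correction.
; The event graph holds only disabled placeholder events, so the Blueprint adds no runtime logic.
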(fn `UserConstructionScript`
  (bind _box (`self.Box`))
  (bind _returnvalue (/ (`self.TileWidth`) 2.0))
  (bind _returnvalue_2 (* (`self.FloorWidth`) (/ (`self.TileWidth`) 2.0)))
  (bind _returnvalue_3 (- (+ (* (/ (`KismetMathLibrary.Conv_IntToDouble` (`self.FloorWidth`)) 2.0) _returnvalue) _returnvalue) 50.0))
  (`BoxComponent.SetBoxExtent` _box (`KismetMathLibrary.MakeVector` _returnvalue_2 _returnvalue_2) true)
  (`SceneComponent.K2_SetRelativeLocation` _box (`KismetMathLibrary.MakeVector` _returnvalue_3 _returnvalue_3) false false))