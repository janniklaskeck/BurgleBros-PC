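; BP_RoomBase is a room Blueprint whose graphs connect its widget components to the room they display.
; On BeginPlay, after the parent call, it hands itself to the item icon list widget in ItemMarkerWidget.
; It then passes itself to the room name widget in RoomTypeWidget to set the room type, stopping if either cast fails.
; The construction script only calls the parent.
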(event `self.ReceiveBeginPlay`
  (`parent.ReceiveBeginPlay`)
  (bind _asw_item_icon_list (cast `/Game/Rooms/ItemMarker/W_ItemIconList` (`WidgetComponent.GetUserWidgetObject` (`self.ItemMarkerWidget`))))
  (set `/Game/Rooms/ItemMarker/W_ItemIconList.Room` self _asw_item_icon_list)
  (bind _asw_room_name (cast `/Game/Rooms/W_RoomName` (`WidgetComponent.GetUserWidgetObject` (`self.RoomTypeWidget`))))
  (`/Game/Rooms/W_RoomName.SetRoomType` _asw_room_name self))

(fn `UserConstructionScript`
  (`parent.UserConstructionScript`))