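; BP_MainGameMode is a game mode Blueprint that sets up the in-game HUD and background music.
; On BeginPlay it creates a W_GameHUD widget, adds it to the viewport, spawns the music as a 2D sound and stores references to both.
; When destroyed, it removes the HUD and stops and destroys the audio component after validity checks.
; Tick only calls the parent.
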(event `self.ReceiveBeginPlay`
  (`parent.ReceiveBeginPlay`)
  (bind _returnvalue (`|CreateWidget` "/Game/UI/W_GameHUD.W_GameHUD_C"))
  (bind _output_get (set `self.GameHUDWidget` _returnvalue))
  (`UserWidget.AddToViewport` _output_get 0)
  (bind _returnvalue_2 (`GameplayStatics.SpawnSound2D` (`self.BGMusic`) 1.0 1.0 0.0 null))
  (set `self.BGMusicComponent` _returnvalue_2))

(event `self.ReceiveTick`
  (params (DeltaSeconds :type "Float (single-precision)"))
  (`parent.ReceiveTick` DeltaSeconds))

(event `self.ReceiveDestroyed`
  (bind _gamehudwidget (`self.GameHUDWidget`))
  (bind _bgmusiccomponent (`self.BGMusicComponent`))
  (`|ExecutionSequence`
    (:`then_0`
      (`/Engine/EditorBlueprintResources/StandardMacros.IsValid` _gamehudwidget
        (:`Is Valid`
          (`Widget.RemoveFromParent` _gamehudwidget))))
    (:`then_1`
      (`/Engine/EditorBlueprintResources/StandardMacros.IsValid` _bgmusiccomponent
        (:`Is Valid`
          (`AudioComponent.Stop` _bgmusiccomponent)
          (`ActorComponent.K2_DestroyComponent` _bgmusiccomponent))))))

(fn `UserConstructionScript`)