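; Game mode for the main menu that swaps between the main menu and the player class selection screen.
; On BeginPlay it shows the main menu, enables the mouse cursor and starts 2D background music.
; Each switch function removes the other widget and creates a fresh one, initializing the class selection widget before display.
; The music component can be faded out through an event and is stopped and destroyed with the game mode.
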(event `self.ReceiveBeginPlay`
  (`self.SwitchToMainMenu`)
  (set `PlayerController.bShowMouseCursor` true (`GameplayStatics.GetPlayerController` 0))
  (bind _returnvalue (`GameplayStatics.SpawnSound2D` "/Game/Sound/Music/Uke_Stanza_-_18_-_Burglar_Bill_Cue.Uke_Stanza_-_18_-_Burglar_Bill_Cue" 1.0 1.0 0.0 null))
  (set `self.BGMusicComponent` _returnvalue))

(event `self.ReceiveDestroyed`
  (bind _bgmusiccomponent (`self.BGMusicComponent`))
  (`/Engine/EditorBlueprintResources/StandardMacros.IsValid` _bgmusiccomponent
    (:`Is Valid`
      (`AudioComponent.Stop` _bgmusiccomponent)
      (`ActorComponent.K2_DestroyComponent` _bgmusiccomponent))))

(event `FadeOutMusic`
  (params (Duration :type "Float (double-precision)"))
  (`AudioComponent.FadeOut` (`self.BGMusicComponent`) Duration 0.0))

(fn `SwitchToChooseClassMenu`
  (`Widget.RemoveFromParent` (`self.MainMenu`))
  (bind _returnvalue (`|CreateWidget` "/Game/UI/MainMenu/W_ChoosePlayerClasses.W_ChoosePlayerClasses_C"))
  (bind _output_get (set `self.ChooseClassesMenu` _returnvalue))
  (`/Game/UI/MainMenu/W_ChoosePlayerClasses.Init` _output_get)
  (`UserWidget.AddToViewport` _output_get 0))

(fn `SwitchToMainMenu`
  (bind _chooseclassesmenu (`self.ChooseClassesMenu`))
  (`/Engine/EditorBlueprintResources/StandardMacros.IsValid` _chooseclassesmenu
    (:`Is Valid`
      (`Widget.RemoveFromParent` _chooseclassesmenu))
    (:`Is Not Valid`
      _))
  (bind _returnvalue (`|CreateWidget` "/Game/UI/MainMenu/W_MainMenu.W_MainMenu_C"))
  (bind _output_get (set `self.MainMenu` _returnvalue))
  (`UserWidget.AddToViewport` _output_get 0))

(fn `UserConstructionScript`)