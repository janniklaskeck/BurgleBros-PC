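; BP_MenuCamera is a camera actor, named for the menu, that circles the world origin.
; Each tick it rotates its location around the world Z axis by Speed times delta time and applies the difference as a world offset to the Camera component.
; It then sets the actor rotation with a look-at toward the world origin, so the view stays aimed at the center.
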(event `self.ReceiveTick`
  (params (DeltaSeconds :type "Float (single-precision)"))
  (`SceneComponent.K2_AddWorldOffset` (`self.Camera`) (- (`KismetMathLibrary.RotateAngleAxis` (`self.K2_GetActorLocation`) (* DeltaSeconds (`self.Speed`)) (0.0 0.0 1.0)) (`self.K2_GetActorLocation`)) false false)
  (`self.K2_SetActorRotation` (`KismetMathLibrary.FindLookAtRotation` (`self.K2_GetActorLocation`) (`KismetMathLibrary.MakeVector` 0.0))))

(fn `UserConstructionScript`)