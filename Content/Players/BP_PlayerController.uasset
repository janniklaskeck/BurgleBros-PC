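; BP_PlayerController is a player controller that binds debug cheat keys for testing.
; F1 toggles CheatsActive once the main game mode has players, enabling number keys that discover all level rooms, add computer tokens, and reset actions or stealth.
; A second set of number keys works only in the editor, independent of that toggle, to inject a specific event, tool or loot item.
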(event `Key|F1`
  (params (Key :type "Key Structure"))
  ;[1 1 1] Cheats
  (:`Pressed`
    (if (> (`KismetArrayLibrary.Array_Length` (`BBMainGameMode.Players` (`BBUtilities.GetMainGameMode`))) 0)
      (set `self.CheatsActive` (not (`self.CheatsActive`))))))

(event `Key|Five`
  (params (Key :type "Key Structure"))
  ;[1 1 1] Cheats
  (:`Pressed`
    (if (`BBUtilities.IsInEditor`)
      (`BBEventLibrary.InsertEventsOnTop` (`|MakeArray` "GoWithYourGut" :!type "EEventType Enum")))))

(event `Key|One`
  (params (Key :type "Key Structure"))
  ;[1 1 1] Cheats
  (:`Pressed`
    (if (`self.CheatsActive`)
      (`BBLevel.DiscoverAllRooms` (`BBUtilities.GetCurrentLevel`)))))

(event `Key|Six`
  (params (Key :type "Key Structure"))
  ;[1 1 1] Cheats
  (:`Pressed`
    (if (`BBUtilities.IsInEditor`)
      (`self.GetTool` (`|MakeArray` "SmokeBomb" :!type "EToolType Enum")))))

(event `Key|Two`
  (params (Key :type "Key Structure"))
  ;[1 1 1] Cheats
  (:`Pressed`
    (if (`self.CheatsActive`)
      (`self.AddComputerTokens` 1))))

(event `Key|Three`
  (params (Key :type "Key Structure"))
  ;[1 1 1] Cheats
  (:`Pressed`
    (if (`self.CheatsActive`)
      (`self.ResetActions`))))

(event `Key|Seven`
  (params (Key :type "Key Structure"))
  ;[1 1 1] Cheats
  (:`Pressed`
    (if (`BBUtilities.IsInEditor`)
      (`self.AddLoot` (`|MakeArray` "Stamp" :!type "ELootType Enum")))))

(event `Key|Four`
  (params (Key :type "Key Structure"))
  ;[1 1 1] Cheats
  (:`Pressed`
    (if (`self.CheatsActive`)
      (`self.ResetStealth`))))

(fn `UserConstructionScript`)